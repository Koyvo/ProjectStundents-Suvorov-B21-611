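; BP_Ball is the Arcanoid ball, handling its own movement, bouncing, scoring and life loss.
; Each Tick it moves with a swept offset and reflects Direction off blocking hits, flattened to Z=0.
; BP_Eraser destroys extra balls; the last ball loses a life, respawns and clears buffs, or pauses into a menu on the final life.
; Hits on actors display-named BP_Generator add score.
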(event EventBeginPlay
  (Variables|Default|SetSpawn%20Location (Transformation|GetActorLocation)))

(event EventTick
  (params (DeltaSeconds :type Float%20%28single-precision%29))
  (bind _sweephitresult (Transformation|AddActorWorldOffset (* (* (Variables|Default|GetDirection) (Variables|Default|GetSpeed)) DeltaSeconds) true))
  (if (.bBlockingHit (Collision|BreakHitResult _sweephitresult))
    (Variables|Default|SetDirection (Math|Vector|MakeVector (.x (Math|Vector|GetReflectionVector (Variables|Default|GetDirection) (.Normal (Collision|BreakHitResult _sweephitresult)))) (.y (Math|Vector|GetReflectionVector (Variables|Default|GetDirection) (.Normal (Collision|BreakHitResult _sweephitresult)))) 0.0))
    (Utilities|Casting|CastToBP_Eraser (.HitActor (Collision|BreakHitResult _sweephitresult))
      (:then
        (bind _outactors (Actor|GetAllActorsOfClass "BP_Ball_C"))
        (if (== (Utilities|Array|Length _outactors) 1)
          (if (== (Variables|Default|GetLives) 1)
            (Game|SetGamePaused true)
            (bind _returnvalue (UserInterface|CreateWidget "/Game/MyLogic/Arcanoid/BP_Menu.BP_Menu_C"))
            (UserInterface|Viewport|AddtoViewport _returnvalue 0)
            (bind _outactors_2 (Actor|GetAllActorsOfClass "/Game/MyLogic/Arcanoid/BP_Buff.BP_Buff_C"))
            (Actor|DestroyActor _outactors_2)
            (Actor|DestroyActor)
            (else
              (bind _output_get (Variables|Default|SetLives (- (Variables|Default|GetLives) 1)))
              (Development|PrintString (Utilities|String|Append "LIVE LEFT: " (Utilities|String|ToString(Integer) _output_get)) true true "(R=1.000000,G=0.000000,B=0.023610,A=1.000000)")
              (Transformation|SetActorLocation (Variables|Default|GetSpawn%20Location) false true)
              (bind _outactors_3 (Actor|GetAllActorsOfClass "/Game/MyLogic/Arcanoid/BP_Buff.BP_Buff_C"))
              (Actor|DestroyActor _outactors_3)))
          (else
            (Actor|DestroyActor))))
      (:CastFailed
        (if (Utilities|Enum|Equal(Enum) (Utilities|GetDisplayName (.HitActor (Collision|BreakHitResult _sweephitresult))) "BP_Generator")
          (bind _output_get_2 (Variables|Default|SetScore (+ (Variables|Default|GetScore) 5)))
          (Development|PrintString (Utilities|String|Append "YOUR SCORE IS " (Utilities|String|ToString(Integer) _output_get_2))))))))

(fn ConstructionScript)
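; BP_Buff is an Arkanoid-style pickup that moves along +Y every tick and applies a random effect when it overlaps BP_Platform.
; SpawnNewBall spawns a BP_Ball at each existing ball, then destroys the pickup.
; ShrinkPlatform halves platform width, sets it to double scale after a Delay inside the loop, then hides and later destroys the pickup.
; Each check re-rolls the random index, so an overlap can do nothing.
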(event Collision|EventActorBeginOverlap
  (params (OtherActor :type Actor%20Object%20Reference))
  (bind _returnvalue (Math|Random|RandomIntegerinRange 0 1))
  (Utilities|Casting|CastToBP_Platform OtherActor)
  (if (Utilities|Enum|Equal(Enum) (Utilities|Array|Get(acopy) (Variables|Default|GetBuffs) _returnvalue) "SpawnNewBall")
    (bind _outactors (Actor|GetAllActorsOfClass "/Game/MyLogic/Arcanoid/BP_Ball.BP_Ball_C"))
    (for _array_element _outactors
      (Game|SpawnActorfromClass "/Game/MyLogic/Arcanoid/BP_Ball.BP_Ball_C" (Math|Transform|MakeTransform (Transformation|GetWorldLocation (Variables|/Game/MyLogic/Arcanoid/BP_Ball.BP_Ball_C|GetSphere _array_element))) "AdjustIfPossibleButAlwaysSpawn" 0 0))
    (Actor|DestroyActor)
    (elif (Utilities|Enum|Equal(Enum) (Utilities|Array|Get(acopy) (Variables|Default|GetBuffs) _returnvalue) "ShrinkPlatform")
      (bind _outactors_2 (Actor|GetAllActorsOfClass "/Game/MyLogic/Arcanoid/BP_Platform.BP_Platform_C"))
      (for _array_element_2 _outactors_2
        (Transformation|SetActorScale3D _array_element_2 "0.500000,1.000000,1.000000")
        (Development|PrintString "U SMOL")
        (Utilities|FlowControl|Delay 1.0)
        (Development|PrintString "U BIG IN...")
        (Transformation|SetActorScale3D _array_element_2 "2.000000,1.000000,1.000000")
        (Development|PrintString "U BIG" true true "(R=0.000000,G=0.660000,B=1.000000,A=1.000000)" 6e+01))
      (Rendering|SetActorHiddenInGame true)
      (Utilities|FlowControl|Delay 2.0)
      (Actor|DestroyActor))))

(event EventTick
  (params (DeltaSeconds :type Float%20%28single-precision%29))
  (Transformation|AddActorWorldOffset "0,5.000000, 0"))

(fn ConstructionScript)
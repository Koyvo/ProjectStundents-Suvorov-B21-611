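; BP_Ball is the ball actor for an Arkanoid game, bouncing off surfaces and keeping the score.
; Each Tick it moves by Direction and Speed with a swept world offset, and on a blocking hit reflects Direction about the hit normal, zeroing Z.
; When the hit actor's display name exactly matches BP_Generator, it adds points to its own Score and prints the total.
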(event EventTick
  (params (DeltaSeconds :type Float%20%28single-precision%29))
  (bind _sweephitresult (Transformation|AddActorWorldOffset (* (* (Variables|Default|GetDirection) (Variables|Default|GetSpeed)) DeltaSeconds) true))
  (if (.bBlockingHit (Collision|BreakHitResult _sweephitresult))
    (Variables|Default|SetDirection (Math|Vector|MakeVector (.x (Math|Vector|GetReflectionVector (Variables|Default|GetDirection) (.Normal (Collision|BreakHitResult _sweephitresult)))) (.y (Math|Vector|GetReflectionVector (Variables|Default|GetDirection) (.Normal (Collision|BreakHitResult _sweephitresult)))) 0.0))
    (if (Utilities|Enum|Equal(Enum) (Utilities|GetDisplayName (.HitActor (Collision|BreakHitResult _sweephitresult))) "BP_Generator")
      (bind _output_get (Variables|Default|SetScore (+ (Variables|Default|GetScore) 5)))
      (Development|PrintString (Utilities|String|Append "YOUR SCORE IS " (Utilities|String|ToString(Integer) _output_get))))))

(fn ConstructionScript)
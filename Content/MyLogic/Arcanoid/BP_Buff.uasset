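; BP_Buff is a pickup for the Arcanoid game that grants its effect when it overlaps BP_Platform.
; It drifts along positive Y by a fixed offset each Tick, without sweep or delta-time scaling.
; If the first Buffs entry is "SpawnNewBall", it spawns a new BP_Ball at every existing ball's location, doubling the count, then destroys itself.
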(event Collision|EventActorBeginOverlap
  (params (OtherActor :type Actor%20Object%20Reference))
  (Utilities|Casting|CastToBP_Platform OtherActor)
  (if (Utilities|Enum|Equal(Enum) (Utilities|Array|Get(acopy) (Variables|Default|GetBuffs)) "SpawnNewBall")
    (bind _outactors (Actor|GetAllActorsOfClass "/Game/MyLogic/Arcanoid/BP_Ball.BP_Ball_C"))
    (for _array_element _outactors
      (Game|SpawnActorfromClass "/Game/MyLogic/Arcanoid/BP_Ball.BP_Ball_C" (Math|Transform|MakeTransform (Transformation|GetWorldLocation (Variables|/Game/MyLogic/Arcanoid/BP_Ball.BP_Ball_C|GetSphere _array_element)) "0, 0, 0" "1.000000,1.000000,1.000000") "AdjustIfPossibleButAlwaysSpawn" 0 0))
    (Actor|DestroyActor)))

(event EventTick
  (params (DeltaSeconds :type Float%20%28single-precision%29))
  (Transformation|AddActorWorldOffset "0,5.000000, 0"))

(fn ConstructionScript)